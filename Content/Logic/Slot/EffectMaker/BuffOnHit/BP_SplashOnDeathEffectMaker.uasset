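; Effect maker for a slot buff-on-hit debuff that makes a target deal splash damage around itself if it dies while affected.
; Setup rolls DPS around a value scaling with the square of base level and a random splash range, deriving damage inversely to that range.
; On spawn it creates and registers a non-stacking SplashDmgOnDeathEffect on the target, then calls the parent.
; A rich-text description reports damage, range and duration.
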(fn `setDescription`
  (bind _returnvalue (`self.cround` (`self.Dmg`)))
  (bind _returnvalue_2 (`self.cround` (`self.Splash`)))
  (set `self.description` (`KismetStringLibrary.Concat_StrStr` "If the target dies while affected by this debuff it deals <YellowReg>" (`KismetStringLibrary.Conv_DoubleToString` _returnvalue) "</> damage in a range of <YellowReg>" (`KismetStringLibrary.Conv_DoubleToString` _returnvalue_2) " </> around the target. Last for a duration of <YellowReg>" (`KismetStringLibrary.Conv_IntToString` (`KismetMathLibrary.FTrunc` (`self.duration`))) "</> seconds.")))

(fn `setup`
  (params (logic :type "LogicEngine Object Reference") (baselevel :type "Float (double-precision)"))
  (locals (dps :type "Float (double-precision)"))
  (bind _baselevel (`local.baselevel`))
  (bind _returnvalue (* (* _baselevel _baselevel) 0.1))
  (bind _returnvalue_2 (* _returnvalue 0.1))
  (bind _returnvalue_3 (`LogicEngine.genNormal` logic _returnvalue _returnvalue_2 _returnvalue_2))
  (set `local.dps` _returnvalue_3)
  (bind _returnvalue_4 (`LogicEngine.genUniform` (`local.logic`) 10.0 100.0))
  (set `self.Splash` _returnvalue_4)
  (set `self.Dmg` (/ (* (`local.dps`) 10.0) _returnvalue_4))
  (set `self.level` (`KismetMathLibrary.FTrunc` (`local.baselevel`)))
  (`self.setDescription` self))

(fn `spawnEffectImpl`
  (params (engine :type "LogicEngine Object Reference") (source :type "TowerEntity Object Reference") (target :type "MobEntity Object Reference"))
  (locals (engine_l :type "LogicEngine Object Reference") (source_l :type "TowerEntity Object Reference") (target_l :type "MobEntity Object Reference"))
  (set `local.engine_l` engine)
  (set `local.source_l` source)
  (set `local.target_l` target)
  (bind _returnvalue (`|GenericCreateObject` "/Script/Cells.SplashDmgOnDeathEffect" (`local.engine_l`)))
  (set `SplashDmgOnDeathEffect._dmg` (`self.Dmg`) _returnvalue)
  (set `SplashDmgOnDeathEffect._splash` (`self.Splash`) _returnvalue)
  (set `TimeBuffEffect._duration` (`self.Duration`) _returnvalue)
  (set `TimeBuffEffect._maxStack` 1 _returnvalue)
  (set `Effect.source` (`local.source_l`) _returnvalue)
  (set `Effect._mobTarget` (`local.target_l`) _returnvalue)
  (`LogicEngine.registerEffect` (`local.engine_l`) _returnvalue)
  (`parent.spawnEffectImpl` (`local.engine_l`) (`local.source_l`) (`local.target_l`)))