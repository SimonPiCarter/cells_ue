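; BP_DirectAttack is an attack slot in the DemoSlot set that directly attacks the closest target to its source.
; SpawnAttack asks the Engine for the closest mob within the source's range, then constructs and registers an AttackEffect for each result, carrying damage, target, source and damage type.
; It returns whether any target was found, and setUpDesc appends the attack text to the basic description.
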(event `setUpDesc`
  (bind _returnvalue (`self.buildBasicDesc`))
  (set `self.description` (`KismetStringLibrary.Concat_StrStr` _returnvalue " Attack closest target.")))

(fn `spawnAttack`
  (params (engine :type "LogicEngine Object Reference") (source :type "TowerEntity Object Reference"))
  (returns (hasAttacked :type Boolean))
  (locals (effect :type "AttackEffect Object Reference"))
  (bind _source (`local.source`))
  (bind _source_2 (`local.source`))
  (bind _effect (`local.effect`))
  ;[1 1 1] spawn attack
  (bind _returnvalue (`LogicEngine.getClosestMobFromPosition` engine (`KismetMathLibrary.Conv_VectorToVector2D` (`Actor.K2_GetActorLocation` _source)) (`TowerEntity.getRange` _source) (`|MakeArray` null :!type "MobEntity Object Reference")))
  (for _array_element _returnvalue
    (bind _returnvalue_2 (`|GenericCreateObject` "/Script/Cells.AttackEffect" engine))
    (bind _output_get (set `local.effect` _returnvalue_2))
    (`LogicEngine.registerEffect` engine _output_get)
    (set `AttackEffect._damage` (`TowerEntity.getDamage` _source_2) _effect)
    (set `Effect._mobTarget` _array_element _effect)
    (set `Effect.source` _source_2 _effect)
    (set `AttackEffect._dmgType` (`self._damageType`) _effect))
  (return (not (`KismetArrayLibrary.Array_IsEmpty` _returnvalue))))

(fn `UserConstructionScript`)