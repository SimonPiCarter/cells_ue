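; Effect maker for a stackable damage-over-time debuff, filed under buff-on-hit slot logic.
; Setup rolls DPS around a value scaling with base level squared, rolls a max stack count, and divides DPS by the unrounded roll to get per-stack damage.
; SpawnEffectImpl constructs a DotEffect with those stats, source and target, registers it with the engine, then calls the parent.
; SetDescription builds rich-text tooltip from damage, duration and stacks.
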(fn `setDescription`
  (bind _returnvalue (`self.cround` (`self.Dmg`)))
  (set `self.description` (`KismetStringLibrary.Concat_StrStr` "Deal <YellowReg>" (`KismetStringLibrary.Conv_DoubleToString` _returnvalue) "</> damage to the target every second for a duration of <YellowReg>" (`KismetStringLibrary.Conv_IntToString` (`KismetMathLibrary.FTrunc` (`self.duration`))) "</> seconds. Can be stacked <YellowReg>" (`KismetStringLibrary.Conv_IntToString` (`self.max_stack`)) "</> times.")))

(fn `setup`
  (params (logic :type "LogicEngine Object Reference") (baselevel :type "Float (double-precision)"))
  (locals (dps :type "Float (double-precision)"))
  (bind _baselevel (`local.baselevel`))
  (bind _returnvalue (* (* _baselevel _baselevel) 0.1))
  (bind _returnvalue_2 (* _returnvalue 0.1))
  (bind _returnvalue_3 (`LogicEngine.genNormal` logic _returnvalue _returnvalue_2 _returnvalue_2))
  (set `local.dps` _returnvalue_3)
  (bind _returnvalue_4 (`LogicEngine.genUniform` (`local.logic`) 1.0 5.0))
  (set `self.max_stack` (`KismetMathLibrary.Round` _returnvalue_4))
  (set `self.Dmg` (/ (`local.dps`) _returnvalue_4))
  (set `self.level` (`KismetMathLibrary.FTrunc` (`local.baselevel`)))
  (`self.setDescription` self))

(fn `spawnEffectImpl`
  (params (engine :type "LogicEngine Object Reference") (source :type "TowerEntity Object Reference") (target :type "MobEntity Object Reference"))
  (locals (engine_l :type "LogicEngine Object Reference") (source_l :type "TowerEntity Object Reference") (target_l :type "MobEntity Object Reference"))
  (set `local.engine_l` engine)
  (set `local.source_l` source)
  (set `local.target_l` target)
  (bind _returnvalue (`|GenericCreateObject` "/Script/Cells.DotEffect" (`local.engine_l`)))
  (set `TimeBuffEffect._duration` (`self.duration`) _returnvalue)
  (set `DotEffect._dmg` (`self.Dmg`) _returnvalue)
  (set `TimeBuffEffect._maxStack` (`self.max_stack`) _returnvalue)
  (set `Effect.source` (`local.source_l`) _returnvalue)
  (set `Effect._mobTarget` (`local.target_l`) _returnvalue)
  (`LogicEngine.registerEffect` (`local.engine_l`) _returnvalue)
  (`parent.spawnEffectImpl` (`local.engine_l`) (`local.source_l`) (`local.target_l`)))