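; Effect maker for slots that applies an on-hit debuff granting the Tower a stacking, timed damage bonus if the target dies while affected.
; SpawnEffectImpl constructs a DmgBonusOnDeathEffect with the buff settings, limits the debuff to one stack, links source and target, registers it with the Engine, then calls the parent.
; SetDescription builds rich-text tooltip copy from the same values, showing the bonus as a percentage.
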(fn `setDescription`
  (bind _returnvalue (`self.cround` (* (`self.Bonus`) 100.0)))
  (set `self.description` (`KismetStringLibrary.Concat_StrStr` "If the target dies while affected by this debuff it increases the damage of the Tower by <YellowReg>" (`KismetStringLibrary.Conv_DoubleToString` _returnvalue) "%</> for a duration of <YellowReg>" (`KismetStringLibrary.Conv_IntToString` (`KismetMathLibrary.FTrunc` (`self.buff_duration`))) "</> seconds. The damage buff can stack <YellowReg>" (`KismetStringLibrary.Conv_IntToString` (`self.max_stack`)) "</> times. The debuff last for a duration of <YellowReg>" (`KismetStringLibrary.Conv_IntToString` (`KismetMathLibrary.FTrunc` (`self.Duration`))) "</> seconds.")))

(fn `spawnEffectImpl`
  (params (engine :type "LogicEngine Object Reference") (source :type "TowerEntity Object Reference") (target :type "MobEntity Object Reference"))
  (locals (engine_l :type "LogicEngine Object Reference") (source_l :type "TowerEntity Object Reference") (target_l :type "MobEntity Object Reference"))
  (set `local.engine_l` engine)
  (set `local.source_l` source)
  (set `local.target_l` target)
  (bind _returnvalue (`|GenericCreateObject` "/Script/Cells.DmgBonusOnDeathEffect" (`local.engine_l`)))
  (`DmgBonusOnDeathEffect.init` _returnvalue (`self.max_stack`) (`self.buff_duration`) (`self.Bonus`))
  (set `TimeBuffEffect._duration` (`self.Duration`) _returnvalue)
  (set `TimeBuffEffect._maxStack` 1 _returnvalue)
  (set `Effect.source` (`local.source_l`) _returnvalue)
  (set `Effect._mobTarget` (`local.target_l`) _returnvalue)
  (`LogicEngine.registerEffect` (`local.engine_l`) _returnvalue)
  (`parent.spawnEffectImpl` (`local.engine_l`) (`local.source_l`) (`local.target_l`)))