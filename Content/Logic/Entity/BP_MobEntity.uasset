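; Mob entity actor that tracks hit points and shows damage numbers when hurt.
; BeginPlay caches ten DamageText widgets from its widget components into an array, which works as a round-robin pool for the damage popups.
; Damage subtracts from Hitpoint and triggers the popup event, with no death check.
; A separate Despawn event hides the cube and disables collision instead of destroying the actor.
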(event `Multi_DamagetextEvent`
  (params (damage :type "Float (double-precision)"))
  ;[1 1 1] Pop Damage Text
  (`/Game/UI/DamageText.PlayDamageText` (`|GetArrayItem` (`self.texts`) (`self.nextText`)) damage)
  (bind _output_get (set `self.nextText` (+ (`self.nextText`) 1)))
  (if (>= _output_get (`KismetArrayLibrary.Array_Length` (`self.texts`)))
    (set `self.nextText` 0)))

(event `self.despawn`
  ;[1 1 1] despawn
  (`SceneComponent.SetHiddenInGame` (`self.Cube`) true true)
  (`self.SetActorEnableCollision` false))

(event `self.damage`
  (params (val :type "Float (single-precision)"))
  ;[1 1 1] damage
  (set `self.hitpoint` (- (`self.hitpoint`) val))
  (`self.Multi_DamagetextEvent` val))

(event `self.ReceiveBeginPlay`
  ;[1 1 1] setup
  (set `self.size` 10.0)
  (set `self.texts` (`|MakeArray` (cast `/Game/UI/DamageText` (`WidgetComponent.GetUserWidgetObject` (`self.DamageText`)) :!pure true) (cast `/Game/UI/DamageText` (`WidgetComponent.GetUserWidgetObject` (`self.DamageText1`)) :!pure true) (cast `/Game/UI/DamageText` (`WidgetComponent.GetUserWidgetObject` (`self.DamageText2`)) :!pure true) (cast `/Game/UI/DamageText` (`WidgetComponent.GetUserWidgetObject` (`self.DamageText3`)) :!pure true) (cast `/Game/UI/DamageText` (`WidgetComponent.GetUserWidgetObject` (`self.DamageText4`)) :!pure true) (cast `/Game/UI/DamageText` (`WidgetComponent.GetUserWidgetObject` (`self.DamageText5`)) :!pure true) (cast `/Game/UI/DamageText` (`WidgetComponent.GetUserWidgetObject` (`self.DamageText6`)) :!pure true) (cast `/Game/UI/DamageText` (`WidgetComponent.GetUserWidgetObject` (`self.DamageText7`)) :!pure true) (cast `/Game/UI/DamageText` (`WidgetComponent.GetUserWidgetObject` (`self.DamageText8`)) :!pure true) (cast `/Game/UI/DamageText` (`WidgetComponent.GetUserWidgetObject` (`self.DamageText9`)) :!pure true))))

(fn `UserConstructionScript`)