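; Controller is a Blueprint that acts as a debug input hook for despawning mobs.
; On BeginPlay it enables input from the first player controller.
; Pressing NumPad 0 queries Logic for all mobs within a small radius of a hardcoded 2D position, despawns each one and prints its index, along with a message confirming the key press.
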(event `Key|NumPadZero`
  (params (Key :type "Key Structure"))
  (:`Pressed`
    (bind _returnvalue (`LogicEngine.getAllMobWithinRadius` (`self.Logic`) (100.0 0.0) 10.0))
    (for (_array_element _array_index) _returnvalue
      (`MobEntity.despawn` _array_element)
      (`KismetSystemLibrary.PrintString` (`KismetStringLibrary.Conv_IntToString` _array_index)))
    (`KismetSystemLibrary.PrintString` (`KismetTextLibrary.Conv_TextToString` "Num 0 pressed"))))

(event `self.ReceiveBeginPlay`
  (`self.EnableInput` (`GameplayStatics.GetPlayerController` 0)))

(fn `UserConstructionScript`)