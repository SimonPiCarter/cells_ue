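; Attack modifier slot logic for a direct attack on the closest mob within the source's range.
; Target selection keeps the source's current target while it is alive and in range, otherwise asks the Engine for the closest mob.
; SpawnAttack creates and registers a primary AttackEffect per target, carrying the source's damage and the damage type, then updates the current target.
; It returns whether any target was found.
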(event `setUpDesc`
  (bind _returnvalue (`self.buildBasicDesc`))
  (set `self.description` (`KismetStringLibrary.Concat_StrStr` _returnvalue " Attack closest target.")))

(fn `selectTarget`
  (params (Source :type "TowerEntity Object Reference") (engine :type "LogicEngine Object Reference"))
  (returns (NewParam :type "Array of MobEntity Object Reference"))
  (bind _source (`local.Source`))
  (bind _source_2 (`local.Source`))
  (bind _returnvalue (`TowerEntity.getRange` _source_2))
  (bind __currenttarget (`TowerEntity._currentTarget` _source_2))
  (if (`KismetSystemLibrary.IsValid` (`TowerEntity._currentTarget` (`local.Source`)))
    (if (and (<= (`KismetMathLibrary.Vector_DistanceSquared` (`Actor.K2_GetActorLocation` _source_2) (`Actor.K2_GetActorLocation` __currenttarget)) (* _returnvalue _returnvalue)) (> (`MobEntity.hitpoint` __currenttarget) 0.0))
      (return (`|MakeArray` (`TowerEntity._currentTarget` (`local.Source`))))
      (else
        _)))
  ;[1 1 1] Find new target
  (bind _returnvalue_2 (`LogicEngine.getClosestMobFromPosition` (`local.engine`) (`KismetMathLibrary.Conv_VectorToVector2D` (`Actor.K2_GetActorLocation` _source)) (`TowerEntity.getRange` _source) (`|MakeArray` null :!type "MobEntity Object Reference")))
  (return _returnvalue_2))

(fn `spawnAttack`
  (params (engine :type "LogicEngine Object Reference") (source :type "TowerEntity Object Reference"))
  (returns (hasAttacked :type Boolean))
  (locals (effect :type "AttackEffect Object Reference"))
  (bind _source (`local.source`))
  (bind _effect (`local.effect`))
  ;[1 1 1] spawn attack
  (bind _newparam (`self.selectTarget` source engine))
  (for _array_element _newparam
    (bind _returnvalue (`|GenericCreateObject` "/Script/Cells.AttackEffect" engine))
    (bind _output_get (set `local.effect` _returnvalue))
    (`LogicEngine.registerEffect` engine _output_get)
    (set `AttackEffect._damage` (`TowerEntity.getDamage` _source) _effect)
    (set `Effect._mobTarget` _array_element _effect)
    (set `Effect.source` _source _effect)
    (set `AttackEffect._dmgType` (`self._damageType`) _effect)
    (set `AttackEffect._primary` true _effect)
    (set `TowerEntity._currentTarget` _array_element (`local.source`)))
  (return (not (`KismetArrayLibrary.Array_IsEmpty` _newparam))))

(fn `UserConstructionScript`)