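; Slot effect maker that applies a combo debuff part to a target, which deals damage once all debuffs in the ID array are present together.
; Setup rolls damage around the squared base level and randomly picks one of three part IDs.
; Spawning registers a single-stack, timed ComboEffect with the engine, then calls the parent implementation.
; A rich-text description lists the required debuffs, damage and duration.
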(fn `setDescription`
  (locals (list :type String))
  (bind _id_array (`self.id array`))
  (bind _list (`local.list`))
  (for (_array_element _array_index) _id_array
    (if (== _array_index 0)
      (bind _returnvalue (`KismetStringLibrary.Concat_StrStr` "<BlueReg>" _array_element "</>"))
      (set `local.list` (`KismetStringLibrary.Concat_StrStr` _list _returnvalue))
      (elif (!= _array_index (- (`KismetArrayLibrary.Array_Length` _id_array) 1))
        (set `local.list` (`KismetStringLibrary.Concat_StrStr` _list ", " _returnvalue))
        (else
          (set `local.list` (`KismetStringLibrary.Concat_StrStr` _list " and  " _returnvalue))))))
  (bind _returnvalue_2 (`self.cround` (`self.dmg`)))
  (set `self.description` (`KismetStringLibrary.Concat_StrStr` "Apply the debuff <BlueReg>" (`self.id`) "</>  to the target. If all debuffs " (`local.list`) " are present at the same time on the target, deals <YellowReg>" (`KismetStringLibrary.Conv_DoubleToString` _returnvalue_2) "</> to the target. Lasts for <YellowReg>" (`KismetStringLibrary.Conv_IntToString` (`KismetMathLibrary.FTrunc` (`self.Duration`))) "</> seconds.")))

(fn `setup`
  (params (logic :type "LogicEngine Object Reference") (baselevel :type "Float (double-precision)"))
  (bind _baselevel (`local.baselevel`))
  (bind _returnvalue (+ (* _baselevel _baselevel) 0.5))
  (bind _returnvalue_2 (* _returnvalue 0.1))
  (bind _returnvalue_3 (`LogicEngine.genNormal` logic _returnvalue _returnvalue_2 _returnvalue_2))
  (set `self.dmg` _returnvalue_3)
  (bind _returnvalue_4 (`LogicEngine.genUniform` (`local.logic`) 0.0 3.0))
  (if (< _returnvalue_4 1.0)
    (set `self.id` "Part1")
    (elif (< _returnvalue_4 2.0)
      (set `self.id` "Part2")
      (else
        (set `self.id` "Part3"))))
  (set `self.level` (`KismetMathLibrary.FTrunc` (`local.baselevel`)))
  (`self.setDescription` self))

(fn `spawnEffectImpl`
  (params (engine :type "LogicEngine Object Reference") (source :type "TowerEntity Object Reference") (target :type "MobEntity Object Reference"))
  (bind _returnvalue (`|GenericCreateObject` "/Script/Cells.ComboEffect" engine))
  (`ComboEffect.init` _returnvalue (`self.id`) (`self.id array`) (`self.dmg`) "Standard")
  (set `TimeBuffEffect._duration` (`self.Duration`) _returnvalue)
  (set `TimeBuffEffect._maxStack` 1 _returnvalue)
  (set `Effect.source` (`local.source`) _returnvalue)
  (set `Effect._mobTarget` (`local.target`) _returnvalue)
  (`LogicEngine.registerEffect` (`local.engine`) _returnvalue)
  (`parent.spawnEffectImpl` (`local.engine`) (`local.source`) (`local.target`)))