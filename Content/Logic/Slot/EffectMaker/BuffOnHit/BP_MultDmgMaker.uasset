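; BP_MultDmgMaker is an on-hit slot effect maker that applies a stackable, timed debuff increasing the damage its target receives.
; Setup derives a total multiplier from a logarithmic curve of base level with normal variance, rolls a random stack cap, divides the multiplier across stacks, then builds the tooltip text.
; SpawnEffectImpl constructs a MultDmgEffect with those values, source and target, registers it with the engine, then calls the parent.
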(fn `setDescription`
  (bind _returnvalue (`self.cround` (* (`self.Mult`) 100.0)))
  (set `self.description` (`KismetStringLibrary.Concat_StrStr` "Increase damage received by the targe by <YellowReg>" (`KismetStringLibrary.Conv_DoubleToString` _returnvalue) "%</> for a duration of <YellowReg>" (`KismetStringLibrary.Conv_IntToString` (`KismetMathLibrary.FTrunc` (`self.duration`))) "</> seconds. Can be stacked <YellowReg>" (`KismetStringLibrary.Conv_IntToString` (`self.max_stack`)) "</> times.")))

(fn `setup`
  (params (logic :type "LogicEngine Object Reference") (baselevel :type "Float (double-precision)"))
  (locals (TargetMult :type "Float (double-precision)"))
  (set `local.TargetMult` (+ (* (/ (`KismetMathLibrary.Log` (+ (/ (`local.baselevel`) 10.0) 0.9) 2.71828) (`KismetMathLibrary.Log` 20.0 2.71828)) 0.6) 0.11))
  (bind _returnvalue (`LogicEngine.genUniform` (`local.logic`) 1.0 5.0))
  (bind _output_get (set `self.max_stack` (`KismetMathLibrary.Round` _returnvalue)))
  (bind _returnvalue_2 (`LogicEngine.genNormal` (`local.logic`) (`local.TargetMult`) 0.05 0.1))
  (set `self.Mult` (/ _returnvalue_2 (`KismetMathLibrary.Conv_IntToDouble` _output_get)))
  (set `self.level` (`KismetMathLibrary.FTrunc` (`local.baselevel`)))
  (`self.setDescription` self))

(fn `spawnEffectImpl`
  (params (engine :type "LogicEngine Object Reference") (source :type "TowerEntity Object Reference") (target :type "MobEntity Object Reference"))
  (locals (engine_l :type "LogicEngine Object Reference") (source_l :type "TowerEntity Object Reference") (target_l :type "MobEntity Object Reference"))
  (set `local.engine_l` engine)
  (set `local.source_l` source)
  (set `local.target_l` target)
  (bind _returnvalue (`|GenericCreateObject` "/Script/Cells.MultDmgEffect" (`local.engine_l`)))
  (set `TimeBuffEffect._duration` (`self.duration`) _returnvalue)
  (set `MultDmgEffect._mult` (`self.Mult`) _returnvalue)
  (set `TimeBuffEffect._maxStack` (`self.max_stack`) _returnvalue)
  (set `Effect.source` (`local.source_l`) _returnvalue)
  (set `Effect._mobTarget` (`local.target_l`) _returnvalue)
  (`LogicEngine.registerEffect` (`local.engine_l`) _returnvalue)
  (`parent.spawnEffectImpl` (`local.engine_l`) (`local.source_l`) (`local.target_l`)))