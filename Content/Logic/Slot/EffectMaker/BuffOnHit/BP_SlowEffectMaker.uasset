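; BP_SlowEffectMaker is an effect maker that applies a stackable slow to a mob target, filed under on-hit buffs.
; SpawnEffectImpl constructs a slow effect, copies in its duration, slow amount, max stack, source and target, registers it with the engine, then calls the parent implementation.
; SetDescription builds rich-text tooltip copy from those values, showing slow as a percentage.
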(fn `setDescription`
  (set `self.description` (`KismetStringLibrary.Concat_StrStr` "Slow target by <YellowReg>" (`KismetStringLibrary.Conv_DoubleToString` (* (`self.slow`) 100.0)) "%</> for a duration of <YellowReg>" (`KismetStringLibrary.Conv_IntToString` (`KismetMathLibrary.FTrunc` (`self.duration`))) "</> seconds. Can be stacked <YellowReg>" (`KismetStringLibrary.Conv_IntToString` (`self.max_stack`)) "</> times.")))

(fn `spawnEffectImpl`
  (params (engine :type "LogicEngine Object Reference") (source :type "TowerEntity Object Reference") (target :type "MobEntity Object Reference"))
  (locals (engine_l :type "LogicEngine Object Reference") (source_l :type "TowerEntity Object Reference") (target_l :type "MobEntity Object Reference"))
  (set `local.engine_l` engine)
  (set `local.source_l` source)
  (set `local.target_l` target)
  (bind _returnvalue (`|GenericCreateObject` "/Script/Cells.SlowEffect" (`local.engine_l`)))
  (set `TimeBuffEffect._duration` (`self.duration`) _returnvalue)
  (set `SlowEffect._slow` (`self.slow`) _returnvalue)
  (set `TimeBuffEffect._maxStack` (`self.max_stack`) _returnvalue)
  (set `Effect.source` (`local.source_l`) _returnvalue)
  (set `Effect._mobTarget` (`local.target_l`) _returnvalue)
  (`LogicEngine.registerEffect` (`local.engine_l`) _returnvalue)
  (`parent.spawnEffectImpl` (`local.engine_l`) (`local.source_l`) (`local.target_l`)))