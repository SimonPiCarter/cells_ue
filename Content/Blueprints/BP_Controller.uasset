(event `Key|I`
  (params (Key :type "Key Structure"))
  (bind _inventorywidget (`self.InventoryWidget`))
  ;[1 1 1] Inventory show up
  (:`Pressed`
    (if (`|EnumEquality` (`Widget.GetVisibility` (`self.InventoryWidget`)) "Visible")
      (`Widget.SetVisibility` _inventorywidget "Hidden")
      (else
        (`Widget.SetVisibility` _inventorywidget "Visible")
        (`/Game/UI/Inventory/Inventory.OpenInventory` _inventorywidget (`/Game/Logic/Engine/BP_LogicEngine.SelectedTower` (`self.Logic`)))))))

(event `self.ReceiveBeginPlay`
  (bind _ascustom_hud (cast `/Game/UI/CustomHUD` (`self.GetHUD` (`GameplayStatics.GetPlayerController` 0))))
  (set `self.customHUD` _ascustom_hud))

(event `Key|LeftMouseButton`
  (params (Key :type "Key Structure"))
  ;[1 1 1] Selection & build
  (:`Pressed`
    (if (`self.BuildMode`)
      (`self.SetBuildMode` (or (`self.IsInputKeyDown` "LeftShift") (`self.IsInputKeyDown` "RightShift")))
      (bind _tower (`/Game/Logic/Engine/BP_LogicEngine.createDemoTower` (`self.Logic`) (`KismetMathLibrary.Conv_VectorToTransform` (`self.TilePosition`))))
      (bind _returnvalue (`LogicEngine.spawnTower` (`self.Logic`) _tower))
      (if (not _returnvalue)
        (`SceneComponent.SetVisibility` (`/Game/Logic/Entity/BP_TowerEntity.DefaultSceneRoot` _tower) false true)
        (`KismetSystemLibrary.PrintString` "Not enough resource"))
      (else
        (`self.SelectTower`)))))

(event `InputVectorAxis|Mouse2D`
  (params (AxisValue :type "Vector Structure"))
  (bind (_bblockinghit _binitialoverlap _time _distance _location _impactpoint _normal _impactnormal _physmat _hitactor) (`GameplayStatics.BreakHitResult` (`self.GetHitResultUnderCursorForObjects` (`|MakeArray` "ObjectTypeQuery1" :!type "EObjectTypeQuery Enum"))))
  (bind _returnvalue (`self.K2_GetActorLocation` _hitactor))
  ;[1 1 1] Scan
  (if (`self.BuildMode`)
    (if _bblockinghit
      (`self.K2_SetActorLocation` (`self.BuildingTower`) _returnvalue false false)
      (set `self.TilePosition` _returnvalue))))

(event `Key|B`
  (params (Key :type "Key Structure"))
  ;[1 1 1] Toogle build mod
  (:`Pressed`
    (`self.SetBuildMode` (not (`self.BuildMode`)))))

(fn `SelectTower`
  (bind _logic (`self.Logic`))
  (bind _ui (`/Game/Logic/Engine/BP_LogicEngine.ui` _logic))
  (bind (_bblockinghit _binitialoverlap _time _distance _location _impactpoint _normal _impactnormal _physmat _hitactor) (`GameplayStatics.BreakHitResult` (`self.GetHitResultUnderCursorForObjects` (`|MakeArray` "ObjectTypeQuery7" :!type "EObjectTypeQuery Enum"))))
  (if _bblockinghit
    (bind _astower_entity (cast `TowerEntity` _hitactor)
      (:`then`
        (bind _output_get (set `/Game/Logic/Engine/BP_LogicEngine.SelectedTower` _astower_entity _logic))
        (`/Game/UI/HeaderUI.TowerSelection_Event` _ui _output_get))
      (:`CastFailed`
        (set `/Game/Logic/Engine/BP_LogicEngine.SelectedTower` null _logic :!label _label)
        (`/Game/UI/HeaderUI.TowerSelection_Event` _ui null)))
    (else
      (goto _label))))

(fn `SetBuildMode`
  (params (`build mode input` :type Boolean))
  (bind _buildingtower (`self.BuildingTower`))
  (bind _cylinder (`/Game/Logic/Entity/BP_TowerEntity.Cylinder` _buildingtower))
  (bind _output_get (set `self.BuildMode` `build mode input`))
  (`SceneComponent.SetVisibility` (`Actor.RootComponent` _buildingtower) _output_get true)
  (if `build mode input`
    (`PrimitiveComponent.SetCollisionEnabled` _cylinder "NoCollision")
    (else
      (`PrimitiveComponent.SetCollisionEnabled` _cylinder "NoCollision"))))

(fn `UserConstructionScript`)